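; Boss actor that swings a wheel continuously from BeginPlay and spawns an explosion on death.
; The RotateWheel timeline lerps the wheel pivot's roll across a fixed arc.
; Each finish waits briefly, then a FlipFlop alternates playing from start and reversing from end, beginning with a second forward play.
; OnDead spawns BP_BossExplosion at the rotate pivot's world location and rotation.
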(event EventBeginPlay
  (bind _rotationamount (Timeline|RotateWheel PlayFromStart)
    (:Update
      (Transformation|SetRelativeRotation (Class|Boss|GetWheelPivot) (Math|Rotator|MakeRotator (Math|Float|Lerp -3e+01 1.8e+02 _rotationamount) 0.0 0.0) false false))
    (:Finished
      (Utilities|FlowControl|Delay 2.0)
      (Utilities|FlowControl|FlipFlop
        (:A
          (Timeline|RotateWheel PlayFromStart))
        (:B
          (Timeline|RotateWheel ReverseFromEnd))))))

(event Collision|EventActorBeginOverlap
  (params (OtherActor :type Actor%20Object%20Reference)))

(event EventTick
  (params (DeltaSeconds :type Float%20%28single-precision%29)))

(event EventOnDead
  (bind _returnvalue (Class|Boss|GetRotatePivot))
  (Game|SpawnActorfromClass "/Game/Blueprints/Boss/vfx/BP_BossExplosion.BP_BossExplosion_C" (Math|Transform|MakeTransform (Transformation|GetWorldLocation _returnvalue) (Transformation|GetWorldRotation _returnvalue) "1.000000,1.000000,1.000000") "Undefined" 0 0))

(fn ConstructionScript)