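; BP_SecurityCamera is a destructible enemy camera with AI sight that pans back and forth.
; The CameraYaw timeline rotates the yaw pivot across RotationRange at MoveSpeed, pausing at each end before a FlipFlop alternates its direction.
; StopMoving freezes the sweep.
; When Health empties, it disables sight, stops panning, spawns explosion effects, physics-simulates its meshes, animates its red light through LightBroke, then destroys itself after a delay.
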(event OnHealthEmpty(Health)
  (bind _returnvalue (Transformation|GetActorLocation))
  (Class|AIPerceptionComponent|SetSenseEnabled (Class|SecurityCamera|GetPerceptionComponent) "/Script/AIModule.AISense_Sight" false)
  (Utilities|FlowControl|Sequence
    (:then_0
      (Components|Timeline|SetPlayRate (Variables|Default|GetCameraYaw) 0.0))
    (:then_1
      (Niagara|SpawnSystematLocation "/Game/VFX/NS_Sparkle.NS_Sparkle" _returnvalue)
      (Effects|SpawnEmitteratLocation "/Game/VFX/P_Explosion.P_Explosion" _returnvalue)
      (for _array_element (Actor|GetComponentsByClass "/Script/Engine.StaticMeshComponent")
        (Physics|SetSimulatePhysics _array_element true)
        (Collision|SetCollisionResponsetoChannel _array_element "ECC_GameTraceChannel1" "ECR_Ignore")))
    (:then_2
      (bind _colormult (Timeline|LightBroke Play)
        (:Update
          (Class|SecurityCamera|SetLightColor (* (Utilities|Struct|MakeLinearColor 1.0 0.0 0.0 1.0) _colormult)))))
    (:then_3
      (Utilities|FlowControl|Delay 5.0)
      (Actor|DestroyActor))))

(event EventBeginPlay
  (bind _rotationrange (Variables|Default|GetRotationRange))
  (Components|Timeline|SetPlayRate (Variables|Default|GetCameraYaw) (Variables|Default|GetMoveSpeed))
  (bind _yaw (Timeline|CameraYaw PlayFromStart)
    (:Update
      (Transformation|SetRelativeRotation (Class|SecurityCamera|GetYawPivot) (Math|Rotator|MakeRotator 0.0 0.0 (Math|Float|Lerp _rotationrange (* _rotationrange -1.0) _yaw)) false false))
    (:Finished
      (Utilities|FlowControl|Delay (Variables|Default|GetPauseDuration))
      (Utilities|FlowControl|FlipFlop
        (:A
          (Timeline|CameraYaw PlayFromStart))
        (:B
          (Timeline|CameraYaw ReverseFromEnd))))))

(event Collision|EventActorBeginOverlap
  (params (OtherActor :type Actor%20Object%20Reference)))

(event EventTick
  (params (DeltaSeconds :type Float%20%28single-precision%29)))

(event EventStopMoving
  (Components|Timeline|SetPlayRate (Variables|Default|GetCameraYaw) 0.0))

(fn ConstructionScript)