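; BP_Box is a box actor that gets knocked away when it takes damage.
; On BeginPlay it binds to its own damage event and passes itself as the Enemy to the WBP_EnemyHealth widget in its EnemyHealth component.
; Damage applies a mass-independent impulse to the static mesh along the damage causer's forward vector, regardless of the damage amount.
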(event Custom|OnTakeAnyDamage_Event_0
  (params (DamagedActor :type Actor%20Object%20Reference) (Damage :type Float%20%28single-precision%29) (DamageType :type Damage%20Type%20Object%20Reference) (InstigatedBy :type Controller%20Object%20Reference) (DamageCauser :type Actor%20Object%20Reference))
  (Physics|AddImpulse (Variables|Default|GetStaticMesh) (* (Transformation|GetActorForwardVector DamageCauser) 1e+03) "None" true))

(event EventBeginPlay
  (EventDispatchers|AssignOnTakeAnyDamage (delegate Custom|OnTakeAnyDamage_Event_0))
  (bind _aswbp_enemy_health (Utilities|Casting|CastToWBP_EnemyHealth (UserInterface|GetUserWidgetObject (Variables|Default|GetEnemyHealth))))
  (Variables|/Game/UI/WBP_EnemyHealth.WBP_EnemyHealth_C|SetEnemy _aswbp_enemy_health self))

(event Collision|EventActorBeginOverlap
  (params (OtherActor :type Actor%20Object%20Reference)))

(event EventTick
  (params (DeltaSeconds :type Float%20%28single-precision%29)))

(fn ConstructionScript)